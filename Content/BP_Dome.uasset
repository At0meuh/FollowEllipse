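; BP_Dome moves a Cube along an upper arc in the XZ plane around its Sphere, following the mouse cursor's direction.
; BeginPlay caches the Sphere's XZ world position as the origin.
; Each Tick deprojects the cursor at spring-arm length and derives its angle from that origin with Atan2.
; Cosine and absolute sine, scaled by the Sphere's bounds, set the Cube's relative location, which is also printed for debugging.
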(event EventTick
  (params (DeltaSeconds :type Float%20%28single-precision%29))
  (bind _returnvalue (Game|GetPlayerController 0))
  (bind _sphere (Variables|Default|GetSphere))
  (bind _springarm (Variables|Default|GetSpringArm))
  (bind _boxextent (Collision|GetComponentBounds _sphere))
  (bind (_locationx _locationy) (Game|Player|GetMousePosition _returnvalue))
  (bind _targetarmlength (Variables|/Script/Engine.SpringArmComponent|GetTargetArmLength _springarm))
  (bind (_x _y _z) (Math|Vector|BreakVector _boxextent))
  (bind _returnvalue_2 (Math|Vector2D|MakeVector2D _locationx _locationy))
  (bind (_worldposition _worlddirection) (Class|GameplayStatics|DeprojectScreentoWorld _returnvalue _returnvalue_2))
  (bind _returnvalue_3 (* _worlddirection _targetarmlength))
  (bind _returnvalue_4 (+ _worldposition _returnvalue_3))
  (Variables|Default|SetMousePosition (Math|Vector2D|MakeVector2D (.x _returnvalue_4) (.z _returnvalue_4)))
  (Variables|Default|SetAngle (+ (Class|KismetMathLibrary|DegAtan2 (.x (- (Variables|Default|GetMousePosition) (Variables|Default|GetMeshOrigine))) (.y (- (Variables|Default|GetMousePosition) (Variables|Default|GetMeshOrigine)))) -9e+01))
  (Transformation|SetRelativeLocation (Variables|Default|GetCube) (Math|Vector|MakeVector (* _x (Math|Trig|Cos(Degrees) (Variables|Default|GetAngle))) 0.0 (Math|Float|Absolute(Float) (* _z (Math|Trig|Sin(Degrees) (* (Variables|Default|GetAngle) -1.0))))) false true)
  (Development|PrintString (Utilities|String|ToString(Vector) (Math|Vector|MakeVector (* _x (Math|Trig|Cos(Degrees) (Variables|Default|GetAngle))) 0.0 (Math|Float|Absolute(Float) (* _z (Math|Trig|Sin(Degrees) (* (Variables|Default|GetAngle) -1.0)))))) true true "(R=0.000000,G=0.660000,B=1.000000,A=1.000000)" 0.0))

(event EventBeginPlay
  (bind _sphere (Variables|Default|GetSphere))
  (bind _returnvalue (Transformation|GetWorldLocation _sphere))
  (Variables|Default|SetMeshOrigine (Math|Vector2D|MakeVector2D (.x _returnvalue) (.z _returnvalue))))

(fn ConstructionScript)